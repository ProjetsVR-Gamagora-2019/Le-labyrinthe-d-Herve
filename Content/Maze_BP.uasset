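; Maze Blueprint is a VR grabbable actor that rotates with the motion controller holding it, without following its position.
; Pickup, called by BP_MotionController, stores the controller component and the per-axis rotation difference between actor and controller.
; While grabbed, Tick adds that offset to the controller's world roll, pitch and yaw to set the actor's rotation.
; Drop clears the grabbed flag to stop the tracking.
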(event `self.ReceiveTick`
  (params (DeltaSeconds :type "Float (single-precision)"))
  (bind (_initdiffrotation_roll _initdiffrotation_pitch _initdiffrotation_yaw) (`KismetMathLibrary.BreakRotator` (`self.initDiffRotation`)))
  (bind (_returnvalue_roll _returnvalue_pitch _returnvalue_yaw) (`KismetMathLibrary.BreakRotator` (`SceneComponent.K2_GetComponentRotation` (`self.grabbingActor`))))
  (if (`self.grabbed`)
    (`self.K2_SetActorRotation` (`KismetMathLibrary.MakeRotator` (+ _returnvalue_roll _initdiffrotation_roll) (+ _returnvalue_pitch _initdiffrotation_pitch) (+ _returnvalue_yaw _initdiffrotation_yaw)))))

(event `/Game/VirtualRealityBP/Blueprints/PickupActorInterface.Pickup`
  (params (AttachTo :type "SceneComponent Object Reference"))
  (bind (_returnvalue_roll _returnvalue_pitch _returnvalue_yaw) (`KismetMathLibrary.BreakRotator` (`self.K2_GetActorRotation`)))
  (bind (_returnvalue_roll_2 _returnvalue_pitch_2 _returnvalue_yaw_2) (`KismetMathLibrary.BreakRotator` (`SceneComponent.K2_GetComponentRotation` (`self.grabbingActor`))))
  (bind _asmotion_controller_component (cast `MotionControllerComponent` AttachTo))
  (set `self.grabbingActor` _asmotion_controller_component)
  (set `self.grabbed` true)
  (set `self.initDiffRotation` (`KismetMathLibrary.MakeRotator` (- _returnvalue_roll _returnvalue_roll_2) (- _returnvalue_pitch _returnvalue_pitch_2) (- _returnvalue_yaw _returnvalue_yaw_2))))

(event `/Game/VirtualRealityBP/Blueprints/PickupActorInterface.Drop`
  (set `self.grabbed` false))

(fn `UserConstructionScript`)